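; Toy tape recorder prop from the RetroKidsToysPack, assembled from separate mesh components on a body mesh.
; The construction script calls a function that attaches the microphone, five transport buttons, cable, door, volume handle and cassette tape to named body sockets, keeping relative transforms.
; It has no runtime logic, as the event graph holds only disabled placeholder events.
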(event EventBeginPlay)

(event Collision|EventActorBeginOverlap
  (params (OtherActor :type Actor%20Object%20Reference)))

(event EventTick
  (params (DeltaSeconds :type Float%20%28single-precision%29)))

(fn ConstructionScript
  (CallFunction|AttatchComponentstoHandles))

(fn AttatchComponentstoHandles
  (bind _toytaperecorder_body (Variables|Default|GetToyTapeRecorder_Body))
  ;[1 1 1] Attach each mesh to the parent mesh using sockets
  (Transformation|AttachComponentToComponent (Variables|Default|GetMicrophone) _toytaperecorder_body "Microphone" "KeepRelative" "KeepRelative" "KeepRelative" true)
  (Transformation|AttachComponentToComponent (Variables|Default|GetButton_Forward) _toytaperecorder_body "Button_Forward" "KeepRelative" "KeepRelative" "KeepRelative" true)
  (Transformation|AttachComponentToComponent (Variables|Default|GetButton_Pause) _toytaperecorder_body "Button_Pause" "KeepRelative" "KeepRelative" "KeepRelative" true)
  (Transformation|AttachComponentToComponent (Variables|Default|GetButton_Play) _toytaperecorder_body "Button_Play" "KeepRelative" "KeepRelative" "KeepRelative" true)
  (Transformation|AttachComponentToComponent (Variables|Default|GetButton_Record) _toytaperecorder_body "Button_Record" "KeepRelative" "KeepRelative" "KeepRelative" true)
  (Transformation|AttachComponentToComponent (Variables|Default|GetButton_Rewind) _toytaperecorder_body "Button_Rewind" "KeepRelative" "KeepRelative" "KeepRelative" true)
  (Transformation|AttachComponentToComponent (Variables|Default|GetCable) _toytaperecorder_body "Cable" "KeepRelative" "KeepRelative" "KeepRelative" true)
  (Transformation|AttachComponentToComponent (Variables|Default|GetDoor) _toytaperecorder_body "Door" "KeepRelative" "KeepRelative" "KeepRelative" true)
  (Transformation|AttachComponentToComponent (Variables|Default|GetVolumeHandle) _toytaperecorder_body "VolumeHandle" "KeepRelative" "KeepRelative" "KeepRelative" true)
  (Transformation|AttachComponentToComponent (Variables|Default|GetCassetteTape) _toytaperecorder_body "CassetteTape" "KeepRelative" "KeepRelative" "KeepRelative" true))