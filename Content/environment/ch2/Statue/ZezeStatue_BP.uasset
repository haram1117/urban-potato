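; Chapter 2 Zeze statue that acts as an ending trigger once it is restored to its golden look.
; ChangeTexture swaps the statue to its clear material and sets a flag that arms the overlap.
; Any actor overlap then shows a closing dialog, fades the camera out after delays and loads MainMenu as a level instance rather than opening it.
; A second dialog about all rides being restored is left unwired.
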(event Custom|ChangeTexture
  (Variables|Default|SetIschangedTexture true)
  (Rendering|Material|SetMaterial (Variables|Default|GetzezeStatue) 0 "/Game/environment/ch2/Statue/ZezeClear_MT.ZezeClear_MT"))

(event EventBeginPlay)

(event Collision|EventActorBeginOverlap
  (params (OtherActor :type Actor%20Object%20Reference))
  (if (Variables|Default|GetIschangedTexture)
    (bind _asmy_player_controller (Utilities|Casting|CastToMyPlayerController (Game|GetPlayerController 0)))
    (Class|NPCDialog|StartDialog (Variables|/Script/UrbanPotato.MyPlayerController|GetdialogWidget _asmy_player_controller) "제제 동상도 금빛으로 돌아왔어! 
제제가 보기 전에 다 고쳐서 다행이야.")
    (Utilities|FlowControl|Delay 4.0)
    (CameraFades|StartCameraFade :self (Game|GetPlayerCameraManager 0) :ToAlpha 1.0 :Duration 5.0)
    (Utilities|FlowControl|Delay 5.0)
    (Class|LevelStreamingDynamic|LoadLevelInstancebySoftObjectPtr "/Game/Base/Maps/MainMenu.MainMenu" "0, 0, 0" "0, 0, 0")))

(event EventTick
  (params (DeltaSeconds :type Float%20%28single-precision%29)))

(fn ConstructionScript)