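; Chapter 2 Ferris wheel puzzle that the player restores by inserting batteries.
; BeginPlay caches every Item_Battery actor, and Interaction checks whether the player's held item is one of them.
; A match removes the item from inventory, increments the count and reveals a battery mesh in the case.
; The second battery starts the looping wheel animation, shows completion dialog and asks the player character to check whether all puzzles are finished.
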(event EventBeginPlay
  (bind _outactors (Actor|GetAllActorsOfClass "/Game/environment/ch2/Battery/Item_Battery.Item_Battery_C"))
  (Variables|Default|Setbattery _outactors))

(event Collision|EventActorBeginOverlap
  (params (OtherActor :type Actor%20Object%20Reference)))

(event EventTick
  (params (DeltaSeconds :type Float%20%28single-precision%29)))

(event EventInteraction
  (bind _asplayer_character (Utilities|Casting|CastToPlayerCharacter (Game|GetPlayerCharacter 0)))
  (for _array_element (Variables|Default|Getbattery)
    (if (== (Variables|/Script/UrbanPotato.PlayerCharacter|GetUsingItem _asplayer_character) _array_element)
      (Rendering|SetVisibility (Variables|Default|GetbatteryCase_MD_pCylinder1) true false)
      (bind _asplayer_character_2 (Utilities|Casting|CastToPlayerCharacter (Game|GetPlayerCharacter 0)))
      (Class|Item|RemovefromInventoryItem _array_element _asplayer_character_2)
      (bind _output_get (Variables|Default|SetbatteryNum (+ (Variables|Default|GetbatteryNum) 1)))
      (if (>= _output_get 2)
        (Rendering|SetVisibility (Variables|Default|GetbatteryCase_MD_pCylinder1_1) true false)
        (Components|Animation|PlayAnimation (Variables|Default|GetferrisWheel_MD_2_) "/Game/environment/ch2/FerrisWheel/ferrisWheel_ANIM_4_.ferrisWheel_ANIM_4_" true)
        (bind _asmy_player_controller (Utilities|Casting|CastToMyPlayerController (Game|GetPlayerController 0)))
        (Class|NPCDialog|StartDialog (Variables|/Script/UrbanPotato.MyPlayerController|GetdialogWidget _asmy_player_controller) "됐어. 모든 놀이기구가 원래대로 돌아왔어! 
이제 제제 동상을 확인해볼까?")
        (bind _asmy_player_character (Utilities|Casting|CastToMyPlayerCharacter (Game|GetPlayerCharacter 0)))
        (Class|PlayerCharacter|CheckAllPuzzlesFinished _asmy_player_character)))))

(fn ConstructionScript)