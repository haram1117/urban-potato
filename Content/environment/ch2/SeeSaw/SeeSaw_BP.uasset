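; SeeSaw_BP is a seesaw puzzle actor that manages the interactable IA_Dice actors in the level, which it gathers on BeginPlay.
; Each EnableDice call assigns an element to the next die by index, reveals it and enables its collision, hiding the seesaw widget once all six are placed.
; DicesWidgetOff triggers the player's all-puzzles-finished check, then turns off every die's widget and unregisters it from player interaction.
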(event Custom|EnableDice
  (Default|SetDiceElement (Utilities|Array|Get(acopy) (Variables|Default|GetDiceList) (Variables|Default|GetdiceIndex)) (Variables|Default|GetdiceIndex))
  (Rendering|SetActorHiddenInGame (Utilities|Array|Get(acopy) (Variables|Default|GetDiceList) (Variables|Default|GetdiceIndex)) false)
  (Collision|SetCollisionEnabled (Variables|/Game/environment/ch2/Dice/BP/IA_Dice.IA_Dice_C|GetSkeletalMesh (Utilities|Array|Get(acopy) (Variables|Default|GetDiceList) (Variables|Default|GetdiceIndex))) "QueryAndPhysics")
  (if (not (Variables|Default|GetAllDiceOnSeeSaw))
    (bind _output_get (Variables|Default|SetdiceIndex (+ (Variables|Default|GetdiceIndex) 1)))
    (if (not (< _output_get 6))
      (Rendering|SetVisibility (Variables|Default|GetWidget) false false)
      (Variables|Default|SetAllDiceOnSeeSaw true))))

(event EventBeginPlay
  (bind _outactors (Actor|GetAllActorsOfClass "/Game/environment/ch2/Dice/BP/IA_Dice.IA_Dice_C"))
  (Variables|Default|SetDiceList _outactors))

(event Collision|EventActorBeginOverlap
  (params (OtherActor :type Actor%20Object%20Reference)))

(event EventTick
  (params (DeltaSeconds :type Float%20%28single-precision%29)))

(event EventDicesWidgetOff
  (bind _asmy_player_character (Utilities|Casting|CastToMyPlayerCharacter (Game|GetPlayerCharacter 0)))
  (Class|PlayerCharacter|CheckAllPuzzlesFinished _asmy_player_character)
  (for _array_element (Variables|Default|GetDiceList)
    (Variables|/Script/UrbanPotato.ActorWithInteractions|SetWidgetOffFlag _array_element true)
    (Rendering|SetVisibility (Variables|/Game/environment/ch2/Dice/BP/IA_Dice.IA_Dice_C|GetWidget _array_element) false false)
    (Variables|/Script/UrbanPotato.ActorWithInteractions|SetisWidgetVisible _array_element false)
    (bind _asplayer_character (Utilities|Casting|CastToPlayerCharacter (Game|GetPlayerCharacter 0)))
    (Class|PlayerCharacter|UnSetInteractActorinBoundary _asplayer_character _array_element)))

(fn ConstructionScript)