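; Chapter 2 seesaw actor that reveals dice one by one, apparently for a puzzle.
; On BeginPlay it caches every IA_Dice in the level, in unsorted GetAllActorsOfClass order.
; Each EnableDice call unhides the next die and enables its mesh collision, advancing an index.
; The sixth call sets AllDiceOnSeeSaw, with the count hard-coded rather than taken from the list.
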(event Custom|EnableDice
  (Rendering|SetActorHiddenInGame (Utilities|Array|Get(acopy) (Variables|Default|GetDiceList) (Variables|Default|GetdiceIndex)) false)
  (Collision|SetCollisionEnabled (Variables|/Game/environment/ch2/BP/IA_dice.IA_Dice_C|GetMesh (Utilities|Array|Get(acopy) (Variables|Default|GetDiceList) (Variables|Default|GetdiceIndex))) "QueryAndPhysics")
  (if (< (+ (Variables|Default|GetdiceIndex) 1) 6)
    (Variables|Default|SetdiceIndex (+ (Variables|Default|GetdiceIndex) 1))
    (else
      (Variables|Default|SetAllDiceOnSeeSaw true))))

(event EventBeginPlay
  (bind _outactors (Actor|GetAllActorsOfClass "/Game/environment/ch2/BP/IA_dice.IA_Dice_C"))
  (for _array_element _outactors
    (bind _asia_dice (Utilities|Casting|CastToIA_Dice _array_element))
    (Utilities|Array|Add (Variables|Default|GetDiceList) _asia_dice)))

(event Collision|EventActorBeginOverlap
  (params (OtherActor :type Actor%20Object%20Reference)))

(event EventTick
  (params (DeltaSeconds :type Float%20%28single-precision%29)))

(fn ConstructionScript)