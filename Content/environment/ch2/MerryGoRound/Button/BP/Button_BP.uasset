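; Interactable button for the Chapter 2 merry-go-round, filled by repeated presses to clear it.
; Each interaction shows the gauge widget and raises ButtonGauge, which drains every frame until full and squashes the button mesh on Z as it rises.
; A full gauge locks the button, hides the widget, shows a clear dialog and calls Clear on MerryGoRound_BP.
; GaugeWidgetOff resets and hides the gauge.
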(event EventBeginPlay
  (bind _returnvalue (Actor|GetActorOfClass "/Game/environment/ch2/MerryGoRound/BP/MerryGoRound_BP.MerryGoRound_BP_C"))
  (Variables|Default|SetMerryGoRound_BP _returnvalue))

(event Collision|EventActorBeginOverlap
  (params (OtherActor :type Actor%20Object%20Reference)))

(event EventTick
  (params (DeltaSeconds :type Float%20%28single-precision%29))
  (Transformation|SetRelativeScale3D (Variables|Default|Getbutton_before_MD_push) (Math|Vector|MakeVector 1.0 1.0 (+ (* (- 1.0 (Variables|Default|GetButtonGauge)) 0.48) 0.52)))
  (if (Variables|Default|GetStartButtonGauge)
    (if (not (Variables|Default|GetIsClear))
      (bind _output_get (Variables|Default|SetButtonGauge (- (Variables|Default|GetButtonGauge) 0.001)))
      (Utilities|FlowControl|Sequence
        (:then_0
          (if (<= _output_get 0.0)
            (Variables|Default|SetButtonGauge 0.0)))
        (:then_1
          (if (>= _output_get 1.0)
            (Variables|Default|SetButtonGauge 1.0)))))))

(event EventInteraction
  (if (not (Variables|Default|GetIsClear))
    (Variables|Default|SetStartButtonGauge true)
    (Rendering|SetVisibility (Variables|Default|GetGaugeWidget) true false)
    (bind _output_get (Variables|Default|SetButtonGauge (+ (Variables|Default|GetButtonGauge) 0.1)))
    (if (>= _output_get 1.0)
      (Variables|Default|SetButtonGauge 1.0)
      (Development|PrintString "Clear")
      (Variables|Default|SetIsClear true)
      (Variables|Default|SetWidgetOffFlag true)
      (Class|ActorwithInteractions|WidgetOff)
      (Rendering|SetVisibility (Variables|Default|GetGaugeWidget) false false)
      (bind _asmy_player_controller (Utilities|Casting|CastToMyPlayerController (Game|GetPlayerController 0)))
      (Class|NPCDialog|StartDialog (Variables|/Script/UrbanPotato.MyPlayerController|GetdialogWidget _asmy_player_controller) "Clear!")
      (Default|Clear (Variables|Default|GetMerryGoRound_BP)))))

(event EventGaugeWidgetOff
  (Variables|Default|SetButtonGauge 0.0)
  (Rendering|SetVisibility (Variables|Default|GetGaugeWidget) false false)
  (Variables|Default|SetStartButtonGauge false))

(fn ConstructionScript)