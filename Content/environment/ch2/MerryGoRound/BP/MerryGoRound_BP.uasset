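; Merry-go-round actor for chapter 2 that starts animating once its puzzle is cleared.
; The Clear event sets IsClear and asks the player character to check whether all puzzles are finished.
; While cleared, Tick spins the rotating platform and bobs odd and even horses in opposite phases, flipping direction at height limits read from horse 2.
; Movement uses fixed per-frame steps, so speed depends on frame rate.
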(event Custom|Clear
  (Variables|Default|SetIsClear true)
  (bind _asmy_player_character (Utilities|Casting|CastToMyPlayerCharacter (Game|GetPlayerCharacter 0)))
  (Class|PlayerCharacter|CheckAllPuzzlesFinished _asmy_player_character))

(event EventBeginPlay)

(event Collision|EventActorBeginOverlap
  (params (OtherActor :type Actor%20Object%20Reference)))

(event EventTick
  (params (DeltaSeconds :type Float%20%28single-precision%29))
  (if (Variables|Default|GetIsClear)
    (Transformation|AddRelativeRotation (Variables|Default|GetMerryGoRound_MD_1__rotation) "0,-0.100000, 0" false false)
    (if (Variables|Default|GetfirstUp)
      (Transformation|AddRelativeLocation (Variables|Default|GetMerryGoRound_MD_1__horse2) "0, 0,0.200000" false false)
      (Transformation|AddRelativeLocation (Variables|Default|GetMerryGoRound_MD_1__horse4) "0, 0,0.200000" false false)
      (Transformation|AddRelativeLocation (Variables|Default|GetMerryGoRound_MD_1__horse6) "0, 0,0.200000" false false)
      (Transformation|AddRelativeLocation (Variables|Default|GetMerryGoRound_MD_1__horse1) "0, 0,-0.200000" false false)
      (Transformation|AddRelativeLocation (Variables|Default|GetMerryGoRound_MD_1__horse3) "0, 0,-0.200000" false false)
      (Transformation|AddRelativeLocation (Variables|Default|GetMerryGoRound_MD_1__horse5) "0, 0,-0.200000" false false)
      (if (>= (.Z (Math|Vector|BreakVector (Variables|/Script/Engine.SceneComponent|GetRelativeLocation (Variables|Default|GetMerryGoRound_MD_1__horse2)))) 25.0)
        (Variables|Default|SetfirstUp false))
      (else
        (Transformation|AddRelativeLocation (Variables|Default|GetMerryGoRound_MD_1__horse2) "0, 0,-0.200000" false false)
        (Transformation|AddRelativeLocation (Variables|Default|GetMerryGoRound_MD_1__horse4) "0, 0,-0.200000" false false)
        (Transformation|AddRelativeLocation (Variables|Default|GetMerryGoRound_MD_1__horse6) "0, 0,-0.200000" false false)
        (Transformation|AddRelativeLocation (Variables|Default|GetMerryGoRound_MD_1__horse1) "0, 0,0.200000" false false)
        (Transformation|AddRelativeLocation (Variables|Default|GetMerryGoRound_MD_1__horse3) "0, 0,0.200000" false false)
        (Transformation|AddRelativeLocation (Variables|Default|GetMerryGoRound_MD_1__horse5) "0, 0,0.200000" false false)
        (if (<= (.Z (Math|Vector|BreakVector (Variables|/Script/Engine.SceneComponent|GetRelativeLocation (Variables|Default|GetMerryGoRound_MD_1__horse2)))) 5.0)
          (Variables|Default|SetfirstUp true))))))

(fn ConstructionScript)